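; AI controller for an enemy that runs BT_Ennemy and tracks the player through AI perception.
; Perception updates write sight stimuli to the blackboard, flag PlayerSeen on a manager once, and restart a one-second looping timer.
; When the timer's counter, never reset here, reaches 60, the player is marked lost and the one-shot flag re-arms.
; A matching hearing handler exists but is never called.
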(event `C_SenseAgeTimer`
  (bind _returnvalue (`KismetSystemLibrary.K2_SetTimerDelegate` (delegate `C_TimerEvent`) 1.0 true)))

(event `C_TimerEvent`
  (bind _timerint (`self.TimerInt`))
  (`/Engine/EditorBlueprintResources/StandardMacros.IncrementInt` _timerint
    (:`  `
      (if (>= _timerint 60)
        (`KismetSystemLibrary.K2_ClearAndInvalidateTimerHandle` (stale `C_SenseAgeTimer` _returnvalue))
        (`self.C_EnnemyLost`)))))

(event `self.AIPerception.OnTargetPerceptionUpdated`
  (params (Actor :type "Actor Object Reference") (Stimulus :type "AIStimulus Structure"))
  ;[1 1 1] Update perception
  (cast `/Game/ThirdPerson/Blueprints/BP_ThirdPersonCharacter` Actor)
  (`self.F_Sight` Stimulus)
  (if (`KismetSystemLibrary.K2_IsValidTimerHandle` (stale `C_SenseAgeTimer` _returnvalue))
    (`KismetSystemLibrary.K2_ClearAndInvalidateTimerHandle` (stale `C_SenseAgeTimer` _returnvalue)))
  (`self.C_SenseAgeTimer`)
  (`/Engine/EditorBlueprintResources/StandardMacros.DoOnce` false :!label _label
    (:`Completed`
      (set `/Game/Ennemis/BP_EnnemyManager.PlayerSeen?` true (`self.ManagerRef`)))))

(event `C_EnnemyLost`
  ;[1 1 1] Player Lost
  (set `/Game/Ennemis/BP_EnnemyManager.PlayerSeen?` false (`self.ManagerRef`))
  (`BlackboardComponent.SetValueAsBool` (`AIBlueprintHelperLibrary.GetBlackboard` null) "bCanSensePlayer" false)
  (goto _label :!via `Reset`))

(event `self.ReceiveBeginPlay`
  (`self.RunBehaviorTree` "/Game/Ennemis/BT_Ennemy.BT_Ennemy"))

(fn `F_Hear`
  (params (Stimulus :type "AIStimulus Structure"))
  (bind _returnvalue (`AIBlueprintHelperLibrary.GetBlackboard` null))
  (bind _returnvalue_2 (`AIPerceptionSystem.GetSenseClassForStimulus` Stimulus))
  (if (== _returnvalue_2 "/Script/AIModule.AISense_Hearing")
    (`BlackboardComponent.SetValueAsBool` _returnvalue "bCanSensePlayer" true)
    (`BlackboardComponent.SetValueAsVector` _returnvalue "LastPlayerLocation" (`.StimulusLocation` (break `AIStimulus` Stimulus)))))

(fn `F_Sight`
  (params (Stimulus :type "AIStimulus Structure"))
  (bind _returnvalue (`AIBlueprintHelperLibrary.GetBlackboard` null))
  (bind _returnvalue_2 (`AIPerceptionSystem.GetSenseClassForStimulus` Stimulus))
  (if (== _returnvalue_2 "/Script/AIModule.AISense_Sight")
    (`BlackboardComponent.SetValueAsBool` _returnvalue "bCanSensePlayer" true)
    (`BlackboardComponent.SetValueAsVector` _returnvalue "LastPlayerLocation" (`.StimulusLocation` (break `AIStimulus` Stimulus)))))

(fn `UserConstructionScript`)