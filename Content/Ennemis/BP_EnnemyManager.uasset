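; BP_EnnemyManager is a box volume that registers the enemies placed inside it and can start them with patrol disabled.
; Shortly after BeginPlay, it passes itself as ManagerRef to each overlapping CH_Ennemy and its controller, setting bDeactivatePatrol in their Blackboards if flagged.
; Player overlap clears the manager's flag without writing to the Blackboards.
; The construction script scales the box from a rounded BoxSize.
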(event `self.ReceiveBeginPlay`
  (`KismetSystemLibrary.Delay` 0.1)
  (bind _output_get (set `self.OverlappingActorsList` (`PrimitiveComponent.GetOverlappingActors` (`self.Box`) "/Game/Ennemis/CH_Ennemy.CH_Ennemy_C")))
  (for _array_element _output_get
    (bind _asch_ennemy (cast `/Game/Ennemis/CH_Ennemy` _array_element))
    (set `/Game/Ennemis/CH_Ennemy.ManagerRef` self _asch_ennemy)
    (bind _aspc_ennemy_controller (cast `/Game/Ennemis/PC_EnnemyController` (`Pawn.GetController` _asch_ennemy)))
    (set `/Game/Ennemis/PC_EnnemyController.ManagerRef` self _aspc_ennemy_controller)
    (if (`self.NeedToDeactivatePatrol?`)
      (`BlackboardComponent.SetValueAsBool` (`AIBlueprintHelperLibrary.GetBlackboard` _asch_ennemy) "bDeactivatePatrol" true))))

(event `self.Box.OnComponentBeginOverlap`
  (params (OverlappedComponent :type "PrimitiveComponent Object Reference") (OtherActor :type "Actor Object Reference") (OtherComp :type "PrimitiveComponent Object Reference") (OtherBodyIndex :type Integer) (bFromSweep :type Boolean) (SweepResult :type "HitResult Structure (by ref)"))
  (if (`self.NeedToDeactivatePatrol?`)
    (cast `/Game/ThirdPerson/Blueprints/BP_ThirdPersonCharacter` OtherActor)
    (set `self.NeedToDeactivatePatrol?` false)))

(fn `UserConstructionScript`
  (bind (_boxsize_x _boxsize_y _boxsize_z) (`KismetMathLibrary.BreakVector` (`self.BoxSize`)))
  (bind _output_get (set `self.BoxSize` (`KismetMathLibrary.MakeVector` (`KismetMathLibrary.Conv_IntToDouble` (`KismetMathLibrary.Round` _boxsize_x)) (`KismetMathLibrary.Conv_IntToDouble` (`KismetMathLibrary.Round` _boxsize_y)) (`KismetMathLibrary.Conv_IntToDouble` (`KismetMathLibrary.Round` _boxsize_z)))))
  (`SceneComponent.SetRelativeScale3D` (`self.Box`) _output_get))