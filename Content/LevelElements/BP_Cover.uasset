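; BP_Cover is a level cover object that builds its mesh and attach points from a size setting.
; Its construction script picks one of three meshes and a point count from CoverSize, scaling the largest variant.
; It then computes evenly spaced, centered rows on both sides of the cover, offset by SpacingWithWall.
; Each position gets a BP_AttachPoint child actor component, stored in a list; BeginPlay and TakeCover are empty.
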(event `self.ReceiveBeginPlay`)

(event `self.TakeCover`)

(fn `F_CheckSize`
  (bind _staticmesh (`self.StaticMesh`))
  (if (`|EnumEquality` (`self.CoverSize`) "NewEnumerator0")
    (set `self.NumberOfAttachPoint` 3)
    (`StaticMeshComponent.SetStaticMesh` (`self.StaticMesh`) "/Game/GameArt/Assets/Environment/SM_Enviro_CoverBois01_Low.SM_Enviro_CoverBois01_Low")
    (elif (`|EnumEquality` (`self.CoverSize`) "NewEnumerator1")
      (set `self.NumberOfAttachPoint` 6)
      (`StaticMeshComponent.SetStaticMesh` (`self.StaticMesh`) "/Game/GameArt/Assets/Environment/SM_Enviro_CoverBois02_Low.SM_Enviro_CoverBois02_Low")
      (else
        (set `self.NumberOfAttachPoint` 10)
        (`StaticMeshComponent.SetStaticMesh` _staticmesh "/Game/GameArt/Assets/Environment/SM_Enviro_CoverTole01_Low.SM_Enviro_CoverTole01_Low")
        (`SceneComponent.SetRelativeScale3D` _staticmesh (2.0 2.0 0.6))))))

(fn `F_CreateAttachPoint`
  (locals (SpacingWithWall :type "Float (double-precision)" :default 40.0))
  (bind (_pointlocation_x _pointlocation_y _pointlocation_z) (`KismetMathLibrary.BreakVector` (`self.PointLocation`)))
  (bind (_pointlocation_x_2 _pointlocation_y_2 _pointlocation_z_2) (`KismetMathLibrary.BreakVector` (`self.PointLocation`)))
  (bind _pointlocation_x_3 (`KismetMathLibrary.BreakVector` (`self.PointLocation`)))
  (bind (_pointlocation_x_4 _pointlocation_y_3 _pointlocation_z_3) (`KismetMathLibrary.BreakVector` (`self.PointLocation`)))
  (bind (_pointlocation_x_5 _pointlocation_y_4 _pointlocation_z_4) (`KismetMathLibrary.BreakVector` (`self.PointLocation`)))
  (set `self.PointLocation` (`KismetMathLibrary.MakeVector` 0.0 (`local.SpacingWithWall`)))
  ;[1 1 1] Even or Odd number of attach point
  (`KismetArrayLibrary.Array_Clear` (`self.AttachPoint`))
  (if (== (mod (`self.NumberOfAttachPoint`) 2) 0)
    ;[1 1 1] Even AttachPoint Number
    (set `self.PointLocation` (`KismetMathLibrary.MakeVector` (+ (- _pointlocation_x_3 (* (/ (`self.NumberOfAttachPoint`) 2) 50)) 25.0) _pointlocation_y_3 _pointlocation_z_3))
    (for _ (range (`self.NumberOfAttachPoint`))
      ;;[1 0.8113 0] Spawn other attach points
      (`KismetArrayLibrary.Array_Add` (`self.AttachPoint`) (`self.PointLocation`))
      (set `self.PointLocation` (`KismetMathLibrary.MakeVector` (+ _pointlocation_x_5 50.0) _pointlocation_y_4 _pointlocation_z_4)))
    ;;[1 0.1039 0] Spawn attach point on the other side
    (for _index (range (`self.NumberOfAttachPoint`))
      (bind (_output_x _output_y _output_z) (`KismetMathLibrary.BreakVector` (`|GetArrayItem` (`self.AttachPoint`) _index)))
      (set `self.PointLocation` (`KismetMathLibrary.MakeVector` _output_x (- _output_y (* (`local.SpacingWithWall`) 2.0)) _output_z))
      (`KismetArrayLibrary.Array_Add` (`self.AttachPoint`) (`self.PointLocation`)))
    (else
      ;[1 1 1] Odd AttachPoint Number
      (set `self.PointLocation` (`KismetMathLibrary.MakeVector` (- _pointlocation_x (* (/ (- (`self.NumberOfAttachPoint`) 1) 2) 50)) _pointlocation_y _pointlocation_z))
      (for _ (range (`self.NumberOfAttachPoint`))
        (`KismetArrayLibrary.Array_Add` (`self.AttachPoint`) (`self.PointLocation`))
        (set `self.PointLocation` (`KismetMathLibrary.MakeVector` (+ _pointlocation_x_2 50.0) _pointlocation_y_2 _pointlocation_z_2)))
      (for _index_2 (range (`self.NumberOfAttachPoint`))
        (bind (_output_x_2 _output_y_2 _output_z_2) (`KismetMathLibrary.BreakVector` (`|GetArrayItem` (`self.AttachPoint`) _index_2)))
        (set `self.PointLocation` (`KismetMathLibrary.MakeVector` _output_x_2 (- _output_y_2 (* (`local.SpacingWithWall`) 2.0)) _output_z_2))
        (`KismetArrayLibrary.Array_Add` (`self.AttachPoint`) (`self.PointLocation`))))))

(fn `UserConstructionScript`
  (`self.F_CheckSize`)
  (`self.F_CreateAttachPoint`)
  (for _array_element (`self.AttachPoint`)
    (bind _returnvalue (`AddComponent|NODE_AddChildActorComponent-1` :`RelativeTransform` (`KismetMathLibrary.MakeTransform` _array_element)))
    (`KismetArrayLibrary.Array_Add` (`self.AttachPointActorList`) _returnvalue)
    (`ChildActorComponent.SetChildActorClass` _returnvalue "/Game/LevelElements/BP_AttachPoint.BP_AttachPoint_C")))