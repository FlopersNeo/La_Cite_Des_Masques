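; Collectable pickup that offers a weapon or ammo to BP_ThirdPersonCharacter on overlap, then destroys itself.
; The construction script picks the mesh from the weapon class, or otherwise from the first Ammo key.
; FAddWeapon adds the class uniquely to the player's WeaponInventory.
; FAddAmmo sums matching amounts into an array from AmmoInventory's values, without explicitly writing back to the map.
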(event `self.Box.OnComponentBeginOverlap`
  (params (OverlappedComponent :type "PrimitiveComponent Object Reference") (OtherActor :type "Actor Object Reference") (OtherComp :type "PrimitiveComponent Object Reference") (OtherBodyIndex :type Integer) (bFromSweep :type Boolean) (SweepResult :type "HitResult Structure (by ref)"))
  (bind _asbp_third_person_character (cast `/Game/ThirdPerson/Blueprints/BP_ThirdPersonCharacter` OtherActor))
  (set `self.PlayerRef` _asbp_third_person_character)
  (`self.F_AddWeapon`)
  (`self.F_AddAmmo`)
  (`self.K2_DestroyActor`))

(fn `F_AddAmmo`
  (bind _ammo (`self.Ammo`))
  (if (`BlueprintMapLibrary.Map_IsNotEmpty` (`self.Ammo`))
    (bind _keys (`BlueprintMapLibrary.Map_Keys` (`/Game/ThirdPerson/Blueprints/BP_ThirdPersonCharacter.AmmoInventory` (`self.PlayerRef`))))
    (for (_array_element _array_index) _keys
      (`|ExecutionSequence`
        (:`then_0`
          (`/Engine/EditorBlueprintResources/StandardMacros.DoOnce` false
            (:`Completed`
              (bind _keys_2 (`BlueprintMapLibrary.Map_Keys` _ammo)))))
        (:`then_1`
          (if (`KismetArrayLibrary.Array_Contains` _keys_2 _array_element)
            (bind _values (`BlueprintMapLibrary.Map_Values` (`/Game/ThirdPerson/Blueprints/BP_ThirdPersonCharacter.AmmoInventory` (`self.PlayerRef`))))
            (`KismetArrayLibrary.Array_Set` _values _array_index (+ (`|GetArrayItem` _values _array_index) (`BlueprintMapLibrary.Map_Find` _ammo _array_element)))))))))

(fn `F_AddWeapon`
  (if (`KismetSystemLibrary.IsValidClass` (`self.Weapon`))
    (`KismetArrayLibrary.Array_AddUnique` (`/Game/ThirdPerson/Blueprints/BP_ThirdPersonCharacter.WeaponInventory` (`self.PlayerRef`)) (`self.Weapon`))
    (return)
    (else
      (return))))

(fn `UserConstructionScript`
  (bind _weapon (`self.Weapon`))
  (bind _staticmesh (`self.StaticMesh`))
  (bind _staticmesh_2 (`self.StaticMesh`))
  (if (`KismetSystemLibrary.IsValidClass` _weapon)
    (if (== _weapon "/Game/ThirdPerson/Blueprints/Weapon/BP_WeaponRifle.BP_WeaponRifle_C")
      (`StaticMeshComponent.SetStaticMesh` _staticmesh (`|GetArrayItem` (`self.MeshList`)))
      (else
        (`StaticMeshComponent.SetStaticMesh` _staticmesh (`|GetArrayItem` (`self.MeshList`) 1))))
    (else
      (bind _keys (`BlueprintMapLibrary.Map_Keys` (`self.Ammo`)))
      (bind _output (`|GetArrayItem` _keys))
      (if (`|EnumEquality` _output "NewEnumerator3")
        (`StaticMeshComponent.SetStaticMesh` _staticmesh_2 (`|GetArrayItem` (`self.MeshList`) 2))
        (`SceneComponent.SetRelativeScale3D` _staticmesh_2 (3.0 3.0 3.0))
        (elif (`|EnumEquality` _output "NewEnumerator4")
          (`StaticMeshComponent.SetStaticMesh` (`self.StaticMesh`) (`|GetArrayItem` (`self.MeshList`) 3))
          (elif (`|EnumEquality` _output "NewEnumerator5")
            (`StaticMeshComponent.SetStaticMesh` (`self.StaticMesh`) (`|GetArrayItem` (`self.MeshList`) 4))))))))