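; Procedural building actor that assembles two opposite facades with roofs in the construction script from instanced modular meshes.
; Module bounds and LastIndesteEnd set column and floor counts, while depth stays fixed regardless of the computed depth count.
; Each ground floor gets one seeded random door, with window modules above and either alternating or optionally corner-capped roof pieces.
; Indices pick meshes and wall/roof materials, and the seed scatters chimneys and antennas on top.
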(fn `UserConstructionScript`
  (locals (Mesh_Leng :type "Float (double-precision)") (Distance_Leng :type "Float (double-precision)") (Distance_Hauteur :type "Float (double-precision)") (Mesh_Hauteur :type "Float (double-precision)") (Mesh_Profondeur :type "Float (double-precision)") (Distance_Profondeur :type "Float (double-precision)"))
  (bind _mesh_leng (`local.Mesh_Leng`))
  (bind _mesh_leng_2 (`local.Mesh_Leng`))
  (bind (_lastindesteend_x _lastindesteend_y _lastindesteend_z) (`KismetMathLibrary.BreakVector` (`self.LastIndesteEnd`)))
  (bind _mesh_leng_3 (`local.Mesh_Leng`))
  (bind _mesh_leng_4 (`local.Mesh_Leng`))
  (bind (_returnvalue_origin _returnvalue_boxextent) (`KismetMathLibrary.BreakBoxSphereBounds` (`StaticMesh.GetBounds` (`self.MeshModule`))))
  (bind _output (`|GetArrayItem` (`self.Toit`) (`self.IDMatToit`)))
  (bind _output_2 (`|GetArrayItem` (`self.Mat`) (`self.IDMat`)))
  (bind _output_3 (`|GetArrayItem` (`self.Mat`) (`self.IDMat`)))
  (bind _returnvalue (- (`self.InstaanceCount`) 1))
  (bind _returnvalue_2 (- (`self.InstaanceCount`) 1))
  (`|ExecutionSequence`
    (:`then_0`
      (`StaticMeshComponent.SetStaticMesh` (`self.Insyance_RDC`) (`self.MeshModule`))
      (`StaticMeshComponent.SetStaticMesh` (`self.Instance_Porte`) (`self.MeshModuleporte`))
      (`StaticMeshComponent.SetStaticMesh` (`self.Instance_Fenetre`) (`|GetArrayItem` (`self.meshConnect`) (`self.IDFenetre`)))
      (`StaticMeshComponent.SetStaticMesh` (`self.Instance_Toit`) (`|GetArrayItem` (`self.meshToit`) (`self.IDToit`)))
      (`StaticMeshComponent.SetStaticMesh` (`self.Instance_ToitFenetre`) (`|GetArrayItem` (`self.meshToit`) (`self.IDToit2`)))
      (`StaticMeshComponent.SetStaticMesh` (`self.Instance_ToitAngle`) (`|GetArrayItem` (`self.meshToitAngle`) (`self.IDToit2Angle`)))
      (`StaticMeshComponent.SetStaticMesh` (`self.Instance_Chemine`) (`|GetArrayItem` (`self.meshChemine`) (`self.IDChemine`)))
      (`StaticMeshComponent.SetStaticMesh` (`self.Instance_Antenet`) (`|GetArrayItem` (`self.meshAntenet`) (`self.IDAnternet`)))
      (`|ExecutionSequence`
        (:`then_0`
          (`PrimitiveComponent.SetMaterialByName` (`self.Insyance_RDC`) "Mur" _output_3))
        (:`then_1`
          (`PrimitiveComponent.SetMaterialByName` (`self.Instance_Fenetre`) "Mur" _output_3))
        (:`then_2`
          (`PrimitiveComponent.SetMaterialByName` (`self.Instance_Toit`) "Mur" _output_3)
          (`|ExecutionSequence`
            (:`then_0`
              (`PrimitiveComponent.SetMaterialByName` (`self.Insyance_RDC`) "Mur2" _output_2))
            (:`then_1`
              (`PrimitiveComponent.SetMaterialByName` (`self.Instance_Fenetre`) "Mur2" _output_2))
            (:`then_2`
              (`PrimitiveComponent.SetMaterialByName` (`self.Instance_Toit`) "Mur2" _output_2)
              (`|ExecutionSequence`
                (:`then_0`
                  (`PrimitiveComponent.SetMaterialByName` (`self.Instance_Toit`) "Toit" _output))
                (:`then_1`
                  (`PrimitiveComponent.SetMaterialByName` (`self.Instance_ToitFenetre`) "Toit" _output))
                (:`then_2`
                  (`PrimitiveComponent.SetMaterialByName` (`self.Instance_ToitAngle`) "Toit" _output))
                (:`then_3`
                  (`PrimitiveComponent.SetMaterialByName` (`self.Instance_Chemine`) "Toit" _output))))
            (:`then_3`
              (`PrimitiveComponent.SetMaterialByName` (`self.Instance_ToitFenetre`) "Mur2" _output_2))
            (:`then_4`
              (`PrimitiveComponent.SetMaterialByName` (`self.Instance_Porte`) "Mur2" _output_2))
            (:`then_5`
              (`PrimitiveComponent.SetMaterialByName` (`self.Instance_Chemine`) "Mur2" _output_2))
            (:`then_6`
              (`PrimitiveComponent.SetMaterialByName` (`self.Instance_ToitAngle`) "Mur2" _output_2))))
        (:`then_3`
          (`PrimitiveComponent.SetMaterialByName` (`self.Instance_ToitFenetre`) "Mur" _output_3))
        (:`then_4`
          (`PrimitiveComponent.SetMaterialByName` (`self.Instance_Porte`) "Mur" _output_3))
        (:`then_5`
          (`PrimitiveComponent.SetMaterialByName` (`self.Instance_Chemine`) "Mur" _output_3))
        (:`then_6`
          (`PrimitiveComponent.SetMaterialByName` (`self.Instance_ToitAngle`) "Mur" _output_3))))
    (:`then_1`
      ;[0.1865 0.0413 0.3073 1 11] distance avec point
      (`|ExecutionSequence`
        (:`then_0`
          (set `local.Mesh_Profondeur` (* (.x _returnvalue_boxextent) -2.0)))
        (:`then_1`
          (set `local.Mesh_Leng` (* (.y _returnvalue_boxextent) 2.0)))
        (:`then_2`
          (set `local.Mesh_Hauteur` (* (.z _returnvalue_boxextent) 2.0)))))
    (:`then_2`
      (`|ExecutionSequence`
        (:`then_0`
          (set `local.Distance_Profondeur` (`KismetMathLibrary.FMax` _lastindesteend_x 1.0)))
        (:`then_1`
          (set `local.Distance_Leng` (`KismetMathLibrary.FMax` _lastindesteend_y 1.0)))
        (:`then_2`
          (set `local.Distance_Hauteur` (`KismetMathLibrary.FMax` _lastindesteend_z 1.0)))))
    (:`then_3`
      (`|ExecutionSequence`
        (:`then_0`
          (set `self.InstaanceCountProfondeur` (`KismetMathLibrary.FFloor` (/ (`local.Distance_Profondeur`) (`local.Mesh_Profondeur`)))))
        (:`then_1`
          (set `self.InstaanceCount` (`KismetMathLibrary.FFloor` (/ (`local.Distance_Leng`) (`local.Mesh_Leng`)))))
        (:`then_2`
          (set `self.InstaanceCountHauteur` (`KismetMathLibrary.FFloor` (/ (`local.Distance_Hauteur`) (`local.Mesh_Hauteur`)))))))
    (:`then_4`
      ;[0.02373 0.04492 0.151] RDC
      (`|ExecutionSequence`
        (:`then_0`
          (set `self.OuLaPorte` (`KismetMathLibrary.RandomIntegerInRangeFromStream` 0 (- (`self.InstaanceCount`) 1) (`self.seed`)))
          (for _index (range (`self.InstaanceCount`))
            (if (== _index (`self.OuLaPorte`))
              (bind _returnvalue_3 (`KismetMathLibrary.MakeTransform` (`KismetMathLibrary.MakeVector` 0.0 (* (`local.Mesh_Leng`) _index))))
              (`InstancedStaticMeshComponent.AddInstance` (`self.Instance_Porte`) _returnvalue_3 false)
              (else
                (`InstancedStaticMeshComponent.AddInstance` (`self.Insyance_RDC`) _returnvalue_3 false)))))
        (:`then_1`
          (set `self.OuLaPorte` (`KismetMathLibrary.RandomIntegerInRangeFromStream` 0 (- (`self.InstaanceCount`) 1) (`self.seed`)))
          (for _index_2 (range (`self.InstaanceCount`))
            (if (== _index_2 (`self.OuLaPorte`))
              (bind _returnvalue_4 (`KismetMathLibrary.MakeTransform` (`KismetMathLibrary.MakeVector` (* (`local.Mesh_Profondeur`) 2.0) (+ (* _mesh_leng_4 _index_2) _mesh_leng_4)) (struct :`Yaw` 180.0)))
              (`InstancedStaticMeshComponent.AddInstance` (`self.Instance_Porte`) _returnvalue_4 false)
              (else
                (`InstancedStaticMeshComponent.AddInstance` (`self.Insyance_RDC`) _returnvalue_4 false)))))))
    (:`then_5`
      ;[0.03022 0.1345 0.151] EtageMillieux
      (`|ExecutionSequence`
        (:`then_0`
          (for _index_3 (range (`self.InstaanceCount`))
            (for _index_4 (range (+ (- (`self.InstaanceCountHauteur`) 2) 1))
              (bind (_returnvalue_x _returnvalue_y _returnvalue_z) (`KismetMathLibrary.BreakVector` (`KismetMathLibrary.MakeVector` 0.0 (* (`local.Mesh_Leng`) _index_3) (* _index_4 (`local.Mesh_Hauteur`)))))
              (`InstancedStaticMeshComponent.AddInstance` (`self.Instance_Fenetre`) (`KismetMathLibrary.MakeTransform` (`KismetMathLibrary.MakeVector` _returnvalue_x _returnvalue_y (+ _returnvalue_z (`local.Mesh_Hauteur`)))) false))))
        (:`then_1`
          (for _index_5 (range (`self.InstaanceCount`))
            (for _index_6 (range (+ (- (`self.InstaanceCountHauteur`) 2) 1))
              (bind (_returnvalue_x_2 _returnvalue_y_2 _returnvalue_z_2) (`KismetMathLibrary.BreakVector` (`KismetMathLibrary.MakeVector` (* (`local.Mesh_Profondeur`) 2.0) (+ _mesh_leng_2 (* _mesh_leng_2 _index_5)) (* _index_6 (`local.Mesh_Hauteur`)))))
              (`InstancedStaticMeshComponent.AddInstance` (`self.Instance_Fenetre`) (`KismetMathLibrary.MakeTransform` (`KismetMathLibrary.MakeVector` _returnvalue_x_2 _returnvalue_y_2 (+ _returnvalue_z_2 (`local.Mesh_Hauteur`))) (struct :`Yaw` 180.0)) false))))))
    (:`then_6`
      ;[0.04568 0.1927 0.09737] toit
      (if (`self.Toit1sur2`)
        ;[0.09421 0.1719 0.04395] toit 2
        (`|ExecutionSequence`
          (:`then_0`
            (for _index_7 (range (`self.InstaanceCount`))
              (if (== (mod _index_7 2) 0)
                (bind (_returnvalue_x_3 _returnvalue_y_3 _returnvalue_z_3) (`KismetMathLibrary.BreakVector` (`KismetMathLibrary.MakeVector` 0.0 (* (`local.Mesh_Leng`) _index_7))))
                (bind _returnvalue_5 (`KismetMathLibrary.MakeTransform` (`KismetMathLibrary.MakeVector` 0.0 _returnvalue_y_3 (+ _returnvalue_z_3 (* (`local.Mesh_Hauteur`) (- (`self.InstaanceCountHauteur`) 0.0))))))
                (`InstancedStaticMeshComponent.AddInstance` (`self.Instance_ToitFenetre`) _returnvalue_5 false)
                (else
                  (`InstancedStaticMeshComponent.AddInstance` (`self.Instance_Toit`) _returnvalue_5 false)))))
          (:`then_1`
            (for _index_8 (range (`self.InstaanceCount`))
              (if (== (mod _index_8 2) 0)
                (bind (_returnvalue_x_4 _returnvalue_y_4 _returnvalue_z_4) (`KismetMathLibrary.BreakVector` (`KismetMathLibrary.MakeVector` (* (`local.Mesh_Profondeur`) 2.0) (+ _mesh_leng (* _mesh_leng _index_8)))))
                (bind _returnvalue_6 (`KismetMathLibrary.MakeTransform` (`KismetMathLibrary.MakeVector` _returnvalue_x_4 _returnvalue_y_4 (+ _returnvalue_z_4 (* (`local.Mesh_Hauteur`) (- (`self.InstaanceCountHauteur`) 0.0)))) (struct :`Yaw` 180.0)))
                (`InstancedStaticMeshComponent.AddInstance` (`self.Instance_ToitFenetre`) _returnvalue_6 false)
                (else
                  (`InstancedStaticMeshComponent.AddInstance` (`self.Instance_Toit`) _returnvalue_6 false))))))
        (else
          (`|ExecutionSequence`
            (:`then_0`
              (for _index_9 (range (+ _returnvalue_2 1))
                (if (`self.ToitAngle`)
                  (bind _returnvalue_7 (== _index_9 _returnvalue_2))
                  (if (or (== _index_9 0) _returnvalue_7)
                    (if _returnvalue_7
                      (bind (_returnvalue_x_5 _returnvalue_y_5 _returnvalue_z_5) (`KismetMathLibrary.BreakVector` (`KismetMathLibrary.MakeVector` 0.0 (* (`local.Mesh_Leng`) _index_9))))
                      (bind _returnvalue_8 (+ _returnvalue_z_5 (* (`local.Mesh_Hauteur`) (- (`self.InstaanceCountHauteur`) 0.0))))
                      (bind _returnvalue_9 (`KismetMathLibrary.MakeTransform` (`KismetMathLibrary.MakeVector` 0.0 _returnvalue_y_5 _returnvalue_8)))
                      (`InstancedStaticMeshComponent.AddInstance` (`self.Instance_ToitAngle`) _returnvalue_9 false)
                      (else
                        (`InstancedStaticMeshComponent.AddInstance` (`self.Instance_ToitAngle`) (`KismetMathLibrary.MakeTransform` (`KismetMathLibrary.MakeVector` -200.0 _returnvalue_y_5 _returnvalue_8) (struct :`Yaw` -90.0)) false)))
                    (else
                      (`InstancedStaticMeshComponent.AddInstance` (`self.Instance_Toit`) _returnvalue_9 false :!label _label)))
                  (else
                    (goto _label)))))
            (:`then_1`
              (for _index_10 (range (+ _returnvalue 1))
                (if (`self.ToitAngle`)
                  (bind _returnvalue_10 (== _index_10 0))
                  (if (or _returnvalue_10 (== _index_10 _returnvalue))
                    (if _returnvalue_10
                      (bind (_returnvalue_x_6 _returnvalue_y_6 _returnvalue_z_6) (`KismetMathLibrary.BreakVector` (`KismetMathLibrary.MakeVector` (* (`local.Mesh_Profondeur`) 2.0) (+ _mesh_leng_3 (* _mesh_leng_3 _index_10)))))
                      (bind _returnvalue_11 (+ _returnvalue_z_6 (* (`local.Mesh_Hauteur`) (- (`self.InstaanceCountHauteur`) 0.0))))
                      (bind _returnvalue_12 (`KismetMathLibrary.MakeTransform` (`KismetMathLibrary.MakeVector` _returnvalue_x_6 _returnvalue_y_6 _returnvalue_11) (struct :`Yaw` 180.0)))
                      (`InstancedStaticMeshComponent.AddInstance` (`self.Instance_ToitAngle`) _returnvalue_12 false)
                      (else
                        (`InstancedStaticMeshComponent.AddInstance` (`self.Instance_ToitAngle`) (`KismetMathLibrary.MakeTransform` (`KismetMathLibrary.MakeVector` (+ _returnvalue_x_6 200.0) _returnvalue_y_6 _returnvalue_11) (struct :`Yaw` 90.0)) false)))
                    (else
                      (`InstancedStaticMeshComponent.AddInstance` (`self.Instance_Toit`) _returnvalue_12 false :!label _label_2)))
                  (else
                    (goto _label_2)))))))))
    (:`then_7`
      ;[0.224 0.2016 0.0713] Antenent
      (for _ (range (`self.NBAntaine`))
        (`InstancedStaticMeshComponent.AddInstance` (`self.Instance_Antenet`) (`KismetMathLibrary.MakeTransform` (`KismetMathLibrary.MakeVector` (`KismetMathLibrary.RandomFloatInRangeFromStream` (* (`local.Mesh_Profondeur`) 0.0) (* (`local.Mesh_Profondeur`) 2.0) (`self.seed`)) (`KismetMathLibrary.RandomFloatInRangeFromStream` 0.0 (* (`local.Mesh_Leng`) (- (`self.InstaanceCount`) 0.0)) (`self.seed`)) (+ 0.0 (* (`local.Mesh_Hauteur`) (- (`self.InstaanceCountHauteur`) 0.0)))) (`KismetMathLibrary.MakeRotator` 0.0 0.0 (`KismetMathLibrary.RandomFloatInRangeFromStream` 0.0 (* (`local.Mesh_Leng`) (- (`self.RotationRandomAntenet`) 0.0)) (`self.seed`)))) false)))
    (:`then_8`
      ;[0.2812 0.114 0.1224] Chemine
      (for _ (range (`self.NBChemine`))
        (`InstancedStaticMeshComponent.AddInstance` (`self.Instance_Chemine`) (`KismetMathLibrary.MakeTransform` (`KismetMathLibrary.MakeVector` (`KismetMathLibrary.RandomFloatInRangeFromStream` (* (`local.Mesh_Profondeur`) -0.5) (* (`local.Mesh_Profondeur`) 1.5) (`self.seed`)) (`KismetMathLibrary.RandomFloatInRangeFromStream` 0.0 (* (`local.Mesh_Leng`) (- (`self.InstaanceCount`) 0.0)) (`self.seed`)) (+ 0.0 (* (`local.Mesh_Hauteur`) (- (`self.InstaanceCountHauteur`) 0.0)))) (`KismetMathLibrary.MakeRotator` 0.0)) false)))))